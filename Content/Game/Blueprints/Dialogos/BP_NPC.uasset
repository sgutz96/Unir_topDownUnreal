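; BP_NPC is a dialogue NPC that advances one line from DialogueTable each time Talk is called.
; It prints the Texto of the CurrentID row, then stores SiguienteID as the next row.
; When no row is found, it clears the UI, then resets to the first ID if IsRepit is set or otherwise destroys itself.
; The WB_Dialog widget creation is disconnected, so lines only appear through PrintText.
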(event EventBeginPlay)

(event Collision|EventActorBeginOverlap
  (params (OtherActor :type Actor%20Object%20Reference)))

(event EventTick
  (params (DeltaSeconds :type Float%20%28single-precision%29)))

(event EventTalk
  ;[0.15 0.15 0.15 0.5] Dialogo
  (bind _returnvalue (Utilities|GetDataTableRow (Variables|Default|GetDialogueTable) (Variables|Default|GetCurrentID))
    (:then
      (Development|PrintText (.Texto (Utilities|Struct|BreakDialogueStruct _returnvalue)))
      (Variables|Default|SetCurrentID (.SiguienteID (Utilities|Struct|BreakDialogueStruct _returnvalue))))
    (:RowNotFound
      (Development|PrintString "No se encontró diálogo")
      (Widget|RemovefromParent (Variables|Default|GetUI))
      (Variables|Default|SetUI 0)
      (if (Variables|Default|GetisRepit)
        (Variables|Default|SetCurrentID "1")
        (else
          (Actor|DestroyActor))))))

(fn ConstructionScript)