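; BP_Enemgo is an enemy that pursues the player and restarts the level on contact with them, by opening TopDownMap.
; From BeginPlay it issues AIMoveTo toward the player character, immediately rotates toward the player controller's location (not the character's), then repeats after a 100-second delay.
; A Box overlap with BP_TopDownCharacterGame triggers the level load.
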(event OnComponentBeginOverlap(Box)
  (params (OverlappedComponent :type Primitive%20Component%20Object%20Reference) (OtherActor :type Actor%20Object%20Reference) (OtherComp :type Primitive%20Component%20Object%20Reference) (OtherBodyIndex :type Integer) (bFromSweep :type Boolean) (SweepResult :type Hit%20Result%20Structure%20%28by%20ref%29))
  (Utilities|Casting|CastToBP_TopDownCharacterGame OtherActor)
  (Game|OpenLevel(byObjectReference) "/Game/TopDown/Maps/TopDownMap.TopDownMap"))

(event EventBeginPlay
  (AI|AIMoveTo self "0, 0, 0" (Game|GetPlayerCharacter 0) 5.0 false :!label _label
    (:then
      (Transformation|SetActorRotation (Math|Rotator|FindLookatRotation (Transformation|GetActorLocation self) (Transformation|GetActorLocation (Game|GetPlayerController 0))))
      (Utilities|FlowControl|Delay 1e+02)
      (goto _label))))

(event Collision|EventActorBeginOverlap
  (params (OtherActor :type Actor%20Object%20Reference)))

(event EventTick
  (params (DeltaSeconds :type Float%20%28single-precision%29)))

(fn ConstructionScript)