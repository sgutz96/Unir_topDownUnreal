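; Player aiming point actor that turns in yaw to face the world point under player 0's mouse cursor.
; Each Tick it traces the cursor on the Visibility channel and derives a look-at rotation, keeping the actor's pitch and roll.
; The look-at feeds RInterpToConstant as Current with no Target, so it steps toward zero rather than easing from the actor's rotation.
; It then stores the Arrow component's world transform in SpawnTransform.
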(event EventBeginPlay)

(event Collision|EventActorBeginOverlap
  (params (OtherActor :type Actor%20Object%20Reference)))

(event EventTick
  (params (DeltaSeconds :type Float%20%28single-precision%29))
  (bind _returnvalue (Transformation|GetActorRotation))
  (Transformation|SetActorRotation (Math|Rotator|MakeRotator (.roll _returnvalue) (.pitch _returnvalue) (.yaw (Class|KismetMathLibrary|RInterptoConstant (Math|Rotator|FindLookatRotation (+ "" "") (- (.ImpactPoint (Collision|BreakHitResult (.HitResult (Game|Player|GetHitResultUnderCursorbyChannel (Game|GetPlayerController 0) "TraceTypeQuery1" true)))) (Transformation|GetActorLocation))) "0, 0, 0" (Utilities|Time|GetWorldDeltaSeconds) (Variables|Default|GetInter%20spead)))))
  (Variables|Default|SetSpawnTransform%20 (Transformation|GetWorldTransform (Variables|Default|GetArrow))))

(fn ConstructionScript)